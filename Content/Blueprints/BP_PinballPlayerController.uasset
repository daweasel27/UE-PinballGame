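; Player controller for a pinball game that turns input into flipper, plunger and table tilt actions and creates the HUD.
; On BeginPlay it finds the plunger and sorts all Flipper actors into left and right lists by flip type.
; Flipper input calls Flip or Flop with side-specific sounds, and plunger input starts or stops charging.
; Tilts spend the game mode's limited TiltCount to push every ball sideways with a mirrored camera shake.
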(event Custom|DetectFlipers
  (bind _outactors (Actor|GetAllActorsOfClass "/Game/Blueprints/Flipper.Flipper_C"))
  (for _array_element _outactors
    (switch Utilities|FlowControl|Switch|SwitchonFlipperType (Variables|/Game/Blueprints/Flipper.Flipper_C|GetFlipType _array_element)
      (:NewEnumerator0
        (Utilities|Array|Add (Variables|Default|GetLeftFlipers) _array_element))
      (:NewEnumerator1
        (Utilities|Array|Add (Variables|Default|GetRightFlipers) _array_element)))))

(event Custom|DetectPlunger
  (bind _outactors (Actor|GetAllActorsOfClass "/Game/Blueprints/BP_pLUNGER.BP_Plunger_C"))
  (Variables|Default|SetPlunger (Utilities|Array|Get(acopy) _outactors)))

(event Custom|CreatePlayerHUD
  (bind _returnvalue (UserInterface|CreateWidget "/Game/Blueprints/PinballHUD.PinballHUD_C"))
  (UserInterface|Viewport|AddtoViewport _returnvalue 0))

(event EventBeginPlay
  (CallFunction|DetectFlipers)
  (CallFunction|DetectPlunger)
  (CallFunction|CreatePlayerHUD))

(event EventTick
  (params (DeltaSeconds :type Float%20%28single-precision%29)))

(event Input|ActionEvents|InputActionLeftFlipper
  (params (Key :type Key%20Structure :default "None"))
  (bind _leftflipers (Variables|Default|GetLeftFlipers))
  (:Pressed
    (for _array_element _leftflipers
      (Default|Flip _array_element)
      (Audio|SpawnSoundAttached "/Game/Assets/Sounds/Pinball_FlipperLeft_Cue.Pinball_FlipperLeft_Cue" (Variables|/Game/Blueprints/Flipper.Flipper_C|GetFlipper _array_element) "None" "0, 0, 0" "0, 0, 0" "KeepRelativeOffset" false 1.0 1.0 0.0 0 0)))
  (:Released
    (for _array_element_2 _leftflipers
      (Default|Flop _array_element_2))))

(event Input|ActionEvents|InputActionRightFlipper
  (params (Key :type Key%20Structure :default "None"))
  (bind _rightflipers (Variables|Default|GetRightFlipers))
  (:Pressed
    (for _array_element _rightflipers
      (Default|Flip _array_element)
      (Audio|PlaySoundatLocation "/Game/Assets/Sounds/Pinball_FlipperRight_Cue.Pinball_FlipperRight_Cue" (.location (Transformation|GetRelativeTransform (Variables|/Game/Blueprints/Flipper.Flipper_C|GetFlipper _array_element))) "0, 0, 0" 1.0 1.0 0.0 0 0 0)))
  (:Released
    (for _array_element_2 _rightflipers
      (Default|Flop _array_element_2))))

(event Input|ActionEvents|InputActionTiltleft
  (params (Key :type Key%20Structure :default "None"))
  (:Pressed
    (CallFunction|Tilt "NewEnumerator0")))

(event Input|ActionEvents|InputActionPlunger
  (params (Key :type Key%20Structure :default "None"))
  (bind _plunger (Variables|Default|GetPlunger))
  (:Pressed
    (bind _asbp_plunger (Utilities|Casting|CastToBP_Plunger _plunger))
    (Default|ChargePlunger _asbp_plunger))
  (:Released
    (bind _asbp_plunger_2 (Utilities|Casting|CastToBP_Plunger _plunger))
    (Default|StopChargePlunger _asbp_plunger_2)))

(event Input|ActionEvents|InputActionTiltRight
  (params (Key :type Key%20Structure :default "None"))
  (:Pressed
    (CallFunction|Tilt "NewEnumerator1")))

(fn ConstructionScript)

(fn Tilt
  (params (Direction :type FlipperType%20Enum :default "NewEnumerator0"))
  (bind _returnvalue (Game|GetPlayerCameraManager 0))
  (bind _returnvalue_2 (Camera|GetCameraRotation _returnvalue))
  (if (> (Variables|/Game/Blueprints/PinballGame.PinballGame_C|GetTiltCount (.AsPinball%20Game (Utilities|Casting|CastToPinballGame (Game|GetGameMode)))) 0)
    (bind _outactors (Actor|GetAllActorsOfClass "/Game/Blueprints/BP_Ball.BP_Ball_C"))
    (if (> (Utilities|Array|Length _outactors) 0)
      (for _array_element _outactors
        (Physics|AddImpulse (Variables|/Game/Blueprints/BP_Ball.BP_Ball_C|GetBall _array_element) (Utilities|Select :Index Direction :NewEnumerator0 "-500.000000, 0, 0" :NewEnumerator1 "500.000000, 0, 0") "None" true)
        (Class|PlayerController|ClientPlayCameraShake "/Game/Blueprints/TiltShake.TiltShake_C" 1.0 "CameraLocal" (Utilities|Select :Index Direction :NewEnumerator0 _returnvalue_2 :NewEnumerator1 (Math|Rotator|CombineRotators _returnvalue_2 "0,180.000000, 0"))))
      (Math|Integer|DecrementInt (Variables|/Game/Blueprints/PinballGame.PinballGame_C|GetTiltCount (.AsPinball%20Game (Utilities|Casting|CastToPinballGame (Game|GetGameMode))))))))